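; BP_Hero is an auto-combat hero pawn that seeks the nearest enemy and pulls in coins.
; A repeating Check sphere-traces nearby objects, picks the closest by line-trace distance, then Attack timeline-rotates and AI-moves toward it, stopping when none are found.
; A one-second timer sends every BP_Coin toward the hero.
; FireBullet spawns BP_InitBullet with camera shake; it and RandomMove have no caller in this graph.
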(event OnComponentBeginOverlap(Sphere)
  (params (OverlappedComponent :type Primitive%20Component%20Object%20Reference) (OtherActor :type Actor%20Object%20Reference) (OtherComp :type Primitive%20Component%20Object%20Reference) (OtherBodyIndex :type Integer) (bFromSweep :type Boolean) (SweepResult :type Hit%20Result%20Structure%20%28by%20ref%29))
  (Utilities|Casting|CastToBP_Coin OtherActor))

(event Custom|RandomMove
  (Variables|Default|SetCanMoveAndAttack true)
  (AI|AIMoveTo self (.RandomLocation (AI|Navigation|GetRandomReachablePointinRadius (Transformation|GetActorLocation) 6e+02 0 0)) 0 5.0 false
    (:OnSuccess
      (Utilities|FlowControl|Delay 0.5))
    (:OnFail
      _))
  (CallFunction|RandomMove))

(event Custom|Check
  (bind _returnvalue (Transformation|GetActorLocation))
  (bind _distancearray (Variables|Default|GetDistanceArray))
  (bind _distanceactormap (Variables|Default|GetDistanceActorMap))
  (bind _minvalue (Math|Float|MinOfFloatArray _distancearray))
  (bind (_value _returnvalue_2) (Utilities|Map|Find _distanceactormap _minvalue))
  (Utilities|FlowControl|Delay 0.05)
  (Utilities|Array|Clear (Variables|Default|GetDistanceArray))
  (Utilities|Map|Clear (Variables|Default|GetDistanceActorMap))
  (bind (_outhits _returnvalue_3) (Collision|MultiSphereTraceForObjects _returnvalue _returnvalue (Variables|Default|GetCheckRadius) (Utilities|Array|MakeArray "ObjectTypeQuery7") false 0 "None"))
  (if _returnvalue_3
    (for _array_element _outhits
      (bind _outhit (Collision|LineTraceForObjects (Transformation|GetActorLocation) (Transformation|GetActorLocation (.HitActor (Collision|BreakHitResult _array_element))) (Utilities|Array|MakeArray "ObjectTypeQuery7") false 0 "None"))
      (Utilities|Array|Add (Variables|Default|GetDistanceArray) (.Distance (Collision|BreakHitResult _outhit)))
      (Utilities|Map|Add (Variables|Default|GetDistanceActorMap) (.Distance (Collision|BreakHitResult _outhit)) (.HitActor (Collision|BreakHitResult _array_element))))
    (if (> (Utilities|Array|Length _distancearray) 0)
      (if _returnvalue_2
        (Variables|Default|SetNearEnemy _value)
        (CallFunction|Attack)
        (else
          (CallFunction|Check :!label _label)))
      (else
        (goto _label)))
    (else
      (Components|Movement|StopMovementImmediately (Variables|Character|GetCharacterMovement))
      (Variables|Default|SetCanMoveAndAttack false)
      (CallFunction|Check))))

(event Custom|Attack
  ;[1 1 1] 攻击
  (Utilities|FlowControl|Sequence
    (:then_0
      (Components|Timeline|SetPlayRate (Variables|Default|GetRotation) 1.0)
      (bind _roationtimline (Timeline|Rotation PlayFromStart)
        (:Update
          (Variables|Default|GetNearEnemy
            (:then
              (Transformation|SetActorRotation (Math|Rotator|Lerp(Rotator) (Transformation|GetActorRotation) (Math|Rotator|FindLookatRotation (Transformation|GetActorLocation) (Transformation|GetActorLocation (Variables|Default|GetNearEnemy))) _roationtimline true)))
            (:else)))))
    (:then_1
      (Variables|Default|SetCanMoveAndAttack true)
      (AI|AIMoveTo self "0, 0, 0" (Variables|Default|GetNearEnemy) 5.0 false
        (:then
          (CallFunction|Check))))))

(event Custom|FireBullet
  (bind _arrow1 (Variables|Default|GetArrow1))
  ;[1 1 1] 发射子弹
  (Game|SpawnActorfromClass "/Game/Havest/BP/BP_InitBullet.BP_InitBullet_C" (Math|Transform|MakeTransform (Transformation|GetWorldLocation _arrow1) (Transformation|GetWorldRotation _arrow1)) "Undefined" "MultiplyWithRoot" 0 0)
  (CallFunction|ShakeScrenn 3.5e+03))

(event Custom|ShakeScrenn
  (params (Radius :type Float%20%28single-precision%29))
  ;[1 1 1] 震屏幕
  (Camera|PlayWorldCameraShake "/Game/Havest/BP/Shake.Shake_C" (Transformation|GetActorLocation) 0.0 Radius))

(event Custom|GetCoins
  (bind _outactors (Actor|GetAllActorsOfClass "/Game/Havest/BP/BP_Coin.BP_Coin_C"))
  (for _array_element _outactors
    (Default|ToTargetPoint _array_element (Transformation|GetWorldLocation (Variables|Character|GetMesh)) self)))

(event EventBeginPlay
  (CallFunction|Check)
  (Utilities|Time|SetTimerbyEvent (delegate Custom|GetCoins) 1.0 true))

(event Collision|EventActorBeginOverlap
  (params (OtherActor :type Actor%20Object%20Reference)))

(event EventTick
  (params (DeltaSeconds :type Float%20%28single-precision%29)))

(fn ConstructionScript
  (|CallParentFunction))