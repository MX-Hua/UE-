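; BP_EnemyDeath is an actor that plays an enemy's death effect, then destroys itself.
; On BeginPlay it enables physics simulation on its skeletal mesh and plays a montage, whose notify starts a timeline driving the material's Fresnel strength.
; That timeline shifts the Fresnel color to dark red at an event key and white on finishing, then a second timeline drives the dissolve parameter before the actor is destroyed.
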(event EventBeginPlay
  (bind _skeletalmesh (Variables|Default|GetSkeletalMesh))
  (Physics|SetSimulatePhysics (Variables|Default|GetSkeletalMesh) true)
  (Animation|Montage|PlayMontage (Variables|Default|GetSkeletalMesh) (Variables|Default|GetMontage%20to%20Play) (Variables|Default|GetPlay%20Rate)
    (:OnNotifyBegin
      (bind _newtrack_0 (Timeline|Timeline PlayFromStart)
        (:Update
          (Rendering|Material|SetScalarParameterValueonMaterials _skeletalmesh "FrenStrenth" _newtrack_0))
        (:Finished
          (Rendering|Material|SetVectorParameterValueonMaterials _skeletalmesh "FrenColor" "1.000000,1.000000,1.000000")
          (bind _time (Timeline|Timeline_1 PlayFromStart)
            (:Update
              (Rendering|Material|SetScalarParameterValueonMaterials (Variables|Default|GetSkeletalMesh) "dissolve" _time))
            (:Finished
              (Actor|DestroyActor))))
        (:ChangeColor
          (Rendering|Material|SetVectorParameterValueonMaterials _skeletalmesh "FrenColor" "0.500000,0.000000,0.000000"))))))

(fn ConstructionScript)