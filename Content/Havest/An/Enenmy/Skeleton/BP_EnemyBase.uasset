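; Base enemy Blueprint that chases the hero through AIMoveTo, reissued every Tick, and handles health, hit reactions and death.
; UpdataBlood adds a randomized damage value to health and spawns a floating number, then triggers Attacked or Death.
; Attacked's montage notify drives material flash, knockback timeline and brief health-bar display, while Tick feeds the bar a lerped trailing fill.
; Death spawns a BP_EnemyDeath stand-in and impulse-launched coins before destroying the actor.
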(event Custom|MoveToRandomTargetPoint
  (bind _returnvalue (Actor|GetActorOfClass (Variables|Default|GetHeroClass)))
  (Utilities|IsValid _returnvalue
    (:Is%20Valid
      (AI|AIMoveTo self "0, 0, 0" _returnvalue 5.0 false))))

(event Custom|UpdateDelayBlood
  ;[1 1 1] 延迟血量
  (Components|Timeline|SetPlayRate (Variables|Default|GetDelayBlood) 1e+01)
  (Variables|Default|SetTempDelayPercent (Variables|Default|GetDelay%20Fill%20Percent))
  (bind _blood (Timeline|DelayBlood PlayFromStart)
    (:Update
      (Variables|Default|SetDelay%20Fill%20Percent (Math|Float|Lerp (Variables|Default|GetTempDelayPercent) (Variables|Default|GetFill%20Percent) _blood)))))

(event Custom|SpawnCoins
  (bind _arrow1 (Variables|Default|GetArrow1))
  (bind _returnvalue (Transformation|GetWorldLocation _arrow1))
  (bind (_x _y _z) (Math|Vector|BreakVector _returnvalue))
  (for _index (range 0 5)
    (bind _returnvalue_2 (Game|SpawnActorfromClass "/Game/Havest/BP/BP_Coin.BP_Coin_C" (Math|Transform|MakeTransform (Math|Vector|MakeVector (Math|Random|RandomFloatinRange (- _x 1e+01) (+ _x 1e+01)) (Math|Random|RandomFloatinRange (- _y 1e+01) (+ _y 1e+01)) _z) "0, 0, 0" (Math|Vector|MakeVector 0.8 0.8 0.8)) "Undefined" "MultiplyWithRoot" 0 0))
    (Default|AddImpulse _returnvalue_2 5e+02 (Transformation|GetWorldLocation (Variables|Default|GetArrow1)))))

(event Custom|UpdataBlood
  (params (DamageValue :type Float%20%28double-precision%29))
  (bind _returnvalue (* DamageValue 2.0))
  (bind _returnvalue_2 (Math|Random|RandomFloatinRange _returnvalue DamageValue))
  ;[1 1 1] 更新血量
  (Game|SpawnActorfromClass "/Game/Havest/BP/BP_AttackedNum.BP_AttackedNum_C" (Math|Transform|MakeTransform (Transformation|GetWorldLocation (Variables|Default|GetWidget)) "0, 0, 0" "1.000000,1.000000,1.000000") "AlwaysSpawn" "MultiplyWithRoot" 0 (Math|Float|Truncate _returnvalue_2) 0)
  (bind _output_get (Variables|Default|SetCurrentBlood (Math|Float|Clamp(Float) (+ (Variables|Default|GetCurrentBlood) _returnvalue_2) 0.0 (Variables|Default|GetMaxBlood))))
  (if (> _output_get 0.0)
    (CallFunction|Attacked)
    (else
      (CallFunction|Death))))

(event Custom|Death
  ;[1 1 1] 死亡actor
  (Game|SpawnActorfromClass "/Game/Havest/An/Enenmy/Skeleton/BP_EnemyDeath.BP_EnemyDeath_C" (Transformation|GetActorTransform) "Undefined" "MultiplyWithRoot" 0 (Variables|Default|GetMontage%20to%20PlayDeath) 1.0 0)
  (CallFunction|SpawnCoins)
  (Actor|DestroyActor))

(event Custom|Attacked
  (bind _widget (Variables|Default|GetWidget))
  ;[1 1 1] 收到攻击
  (Animation|Montage|PlayMontage (Variables|Character|GetMesh) (Variables|Default|GetMontage%20to%20Play) (Variables|Default|GetPlay%20Rate)
    (:OnNotifyBegin
      (Utilities|FlowControl|Sequence
        (:then_0
          (CallFunction|Fren))
        (:then_1
          (CallFunction|MovetoBackward))
        (:then_2
          (Development|SetHiddeninGame _widget false false)
          (Utilities|FlowControl|Delay 1.0)
          (Development|SetHiddeninGame _widget true false))))))

(event Custom|MoveToBackward
  (bind _returnvalue (Transformation|GetActorLocation))
  ;[1 1 1] 被击后退
  (Components|Timeline|SetPlayRate (Variables|Default|GetMoveBackward) 1e+01)
  (bind _newtrack_0 (Timeline|MoveBackward PlayFromStart)
    (:Update
      (Transformation|SetActorLocation (Math|Vector|Lerp(Vector) _returnvalue (- _returnvalue (* (Transformation|GetActorForwardVector) 20)) _newtrack_0) false false))))

(event Custom|Fren
  ;[1 1 1] Fren
  (bind _newtrack_0 (Timeline|FrenStrenth PlayFromStart)
    (:Update
      (Rendering|Material|SetScalarParameterValueonMaterials (Variables|Character|GetMesh) "FrenStrenth" _newtrack_0))
    (:Finished
      (Rendering|Material|SetVectorParameterValueonMaterials (Variables|Character|GetMesh) "FrenColor" "1.000000,1.000000,1.000000"))
    (:ChangeColor
      (Rendering|Material|SetVectorParameterValueonMaterials (Variables|Character|GetMesh) "FrenColor" "1.000000,0.000000,0.000000"))))

(event EventBeginPlay
  ;[1 1 1] 初始化血量为最大血量
  (Variables|Default|SetCurrentBlood (Variables|Default|GetMaxBlood))
  (Development|SetHiddeninGame (Variables|Default|GetWidget) true false))

(event Collision|EventActorBeginOverlap
  (params (OtherActor :type Actor%20Object%20Reference)))

(event EventTick
  (params (DeltaSeconds :type Float%20%28single-precision%29))
  ;[1 1 1] 更新延迟血量
  (bind _asumg_blood (Utilities|Casting|CastToUMG_Blood (UserInterface|GetWidget (Variables|Default|GetWidget))))
  (Variables|Default|SetFill%20Percent (/ (Variables|Default|GetCurrentBlood) (Variables|Default|GetMaxBlood)))
  (CallFunction|UpdateDelayBlood)
  (Default|UpdateBlood _asumg_blood (Variables|Default|GetFill%20Percent) (Variables|Default|GetDelay%20Fill%20Percent) (Variables|Default|GetScale))
  (CallFunction|MovetoRandomTargetPoint))

(fn ConstructionScript
  (|CallParentFunction))